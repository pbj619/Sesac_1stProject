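; BP_MonsterController is the AI controller that drives monster pawns.
; On possess it loads the BP_MonsterBB blackboard, zeroes the patrol time key and stores the pawn's spawn position as the start location key.
; It then runs the BP_MonsterBT behavior tree, which handles the monster's decisions from that blackboard data.
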(event `self.ReceivePossess`
  (params (PossessedPawn :type "Pawn Object Reference"))
  (`|ExecutionSequence`
    (:`then_0`
      (`self.UseBlackboard` "/Game/WorkSpace/Monster/AI/BP_MonsterBB.BP_MonsterBB")
      (`BlackboardComponent.SetValueAsFloat` (`self.Blackboard`) (`self.PatrolTime KeyName`) 0.0)
      (`BlackboardComponent.SetValueAsVector` (`self.Blackboard`) (`self.StartLocationKeyName`) (`self.K2_GetActorLocation` (`self.K2_GetPawn`))))
    (:`then_1`
      (`self.RunBehaviorTree` "/Game/WorkSpace/Monster/AI/BP_MonsterBT.BP_MonsterBT"))))

(fn `UserConstructionScript`)