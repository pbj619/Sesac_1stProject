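; BP_Monster1 is a monster character Blueprint that manages its behavior state and matching movement speed.
; SetState ignores any change once the monster is Dead; otherwise it stores the new state and calls CallStateChangedEvent with it.
; It then sets the walk speed, slower for Locomotion, faster for Chase, and zero for Attack and Dead.
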(event `SetState`
  (params (NewState :type "/Game/WorkSpace/Monster/EMonster1State Enum" :default "NewEnumerator0"))
  (bind _charactermovement (`self.CharacterMovement`))
  (if (not (`|EnumEquality` (`self.State`) "NewEnumerator3"))
    (bind _output_get (set `self.State` NewState))
    (`self.StateChangedEvent` _output_get)
    (switch `/Game/WorkSpace/Monster/EMonster1State` (`self.State`)
      (:`NewEnumerator0`
        (set `CharacterMovementComponent.MaxWalkSpeed` 250.0 _charactermovement))
      (:`NewEnumerator1`
        (set `CharacterMovementComponent.MaxWalkSpeed` 500.0 _charactermovement))
      (:`NewEnumerator2`
        (set `CharacterMovementComponent.MaxWalkSpeed` 0.0 _charactermovement :!label _label))
      (:`NewEnumerator3`
        (goto _label)))))

(fn `UserConstructionScript`)