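; BP_Player is the player character, handling axis movement, jump, hold-to-sprint, hold-to-crouch and firing.
; Movement follows control yaw, and Fire spawns a BP_Bullet at the FirePosition transform.
; Tab toggles target lock: a debug-drawn sphere trace along the camera's forward vector stores a hit Pawn as HitTarget, or clears it.
; While HitTarget is valid, Tick turns control rotation toward it.
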(event `InputAxis|moveforward`
  (params (AxisValue :type "Float (single-precision)"))
  ;[1 1 1] 컨트롤
  (`self.AddMovementInput` (`KismetMathLibrary.GetForwardVector` (`KismetMathLibrary.MakeRotator` 0.0 0.0 (.yaw (`self.GetControlRotation`)))) AxisValue))

(event `self.ReceiveTick`
  (params (DeltaSeconds :type "Float (single-precision)"))
  (`self.hit target`
    (:`then`
      (`Controller.SetControlRotation` (`self.GetController`) (`KismetMathLibrary.FindLookAtRotation` (`self.K2_GetActorLocation`) (`self.K2_GetActorLocation` (`self.hit target`)))))
    (:`else`)))

(event `InputAxis|LeftRight`
  (params (AxisValue :type "Float (single-precision)"))
  ;[1 1 1] 컨트롤
  (`self.AddMovementInput` (`KismetMathLibrary.GetRightVector` (`KismetMathLibrary.MakeRotator` 0.0 0.0 (.yaw (`self.GetControlRotation`)))) AxisValue))

(event `InputAction|jump`
  (params (Key :type "Key Structure"))
  ;[1 1 1] 점프, 달리기, 앉기
  (:`Pressed`
    (`self.Jump`))
  (:`Released`
    (`self.StopJumping`)))

(event `InputAction|sprint`
  (params (Key :type "Key Structure"))
  (bind _charactermovement (`self.CharacterMovement`))
  ;[1 1 1] 점프, 달리기, 앉기
  (:`Pressed`
    (set `CharacterMovementComponent.MaxWalkSpeed` 1000.0 _charactermovement))
  (:`Released`
    (set `CharacterMovementComponent.MaxWalkSpeed` 600.0 _charactermovement)))

(event `InputAction|crouch`
  (params (Key :type "Key Structure"))
  ;[1 1 1] 점프, 달리기, 앉기
  (:`Pressed`
    (`self.Crouch`))
  (:`Released`
    (`self.UnCrouch`)))

(event `InputAction|tab`
  (params (Key :type "Key Structure"))
  (bind _returnvalue (`self.K2_GetActorLocation`))
  (:`Pressed`
    (`/Engine/EditorBlueprintResources/StandardMacros.FlipFlop`
      (:`A`
        (set `self.targetLock` true)
        (bind (_outhit _returnvalue_2) (`KismetSystemLibrary.SphereTraceSingleForObjects` :`Start` _returnvalue :`End` (+ _returnvalue (* (`KismetMathLibrary.GetForwardVector` (`SceneComponent.K2_GetComponentRotation` (`self.Camera`))) (`self.??`))) :`ObjectTypes` (`|MakeArray` "ObjectTypeQuery3" :!type "EObjectTypeQuery Enum") :`DrawDebugType` "ForDuration"))
        (if _returnvalue_2
          (set `self.hit target` (`.HitActor` (`GameplayStatics.BreakHitResult` _outhit)))))
      (:`B`
        (set `self.targetLock` false)
        (set `self.hit target` null)))))

(event `InputAction|Fire`
  (params (Key :type "Key Structure"))
  ;[1 1 1] 총을 쏘다!
  (:`Pressed`
    (`|SpawnActorFromClass` "/Game/BP_Player/BP_Bullet.BP_Bullet_C" (`SceneComponent.K2_GetComponentToWorld` (`self.FirePosition`)) "AlwaysSpawn" "MultiplyWithRoot" null null)))

(fn `UserConstructionScript`)